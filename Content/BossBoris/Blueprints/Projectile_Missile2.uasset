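; Homing missile projectile in the Boris boss content that explodes on contact or on a timeout.
; After a short delay it turns on strong ProjectileMovement homing toward player 0's root component.
; Sphere overlaps with anything except AdvancedBorisAI_BP spawn an actor, set HasExploded and destroy the missile.
; If it has not exploded a few seconds after homing starts, it spawns an Explosion and destroys itself.
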(event OnComponentBeginOverlap(Sphere)
  (params (OverlappedComponent :type Primitive%20Component%20Object%20Reference) (OtherActor :type Actor%20Object%20Reference) (OtherComp :type Primitive%20Component%20Object%20Reference) (OtherBodyIndex :type Integer) (bFromSweep :type Boolean) (SweepResult :type Hit%20Result%20Structure%20%28by%20ref%29))
  (Utilities|Casting|CastToAdvancedBorisAI_BP OtherActor
    (:CastFailed
      (Utilities|FlowControl|DoOnce false
        (:Completed
          (Game|SpawnActorfromClass "/Game/BossBoris/Blueprints/Explosion.Explosion_C" (Transformation|GetWorldTransform (Variables|Default|GetDefaultSceneRoot)) "AlwaysSpawn" 0 0)
          (Variables|Default|SetHasExploded true)
          (Actor|DestroyActor))))))

(event EventBeginPlay
  (bind _projectilemovement (Variables|Default|GetProjectileMovement))
  (Utilities|FlowControl|Delay 0.4)
  (Variables|/Script/Engine.ProjectileMovementComponent|SetHomingTargetComponent _projectilemovement (Variables|/Script/Engine.Actor|GetRootComponent (Game|GetPlayerCharacter 0)))
  (Variables|/Script/Engine.ProjectileMovementComponent|SetbIsHomingProjectile _projectilemovement true)
  (Variables|/Script/Engine.ProjectileMovementComponent|SetHomingAccelerationMagnitude _projectilemovement 1e+04)
  (Utilities|FlowControl|Delay 3.0)
  (if (not (Variables|Default|GetHasExploded))
    (Utilities|FlowControl|DoOnce false
      (:Completed
        (Game|SpawnActorfromClass "/Game/BossBoris/Blueprints/Explosion.Explosion_C" (Transformation|GetWorldTransform (Variables|Default|GetDefaultSceneRoot)) "AlwaysSpawn" 0 0)
        (Actor|DestroyActor)))))

(fn ConstructionScript)